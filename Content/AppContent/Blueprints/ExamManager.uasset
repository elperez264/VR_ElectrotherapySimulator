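; Exam manager that quizzes the player on treatment settings for the Magneto and Micro devices.
; Starting or finishing the exam notifies Russ, Magneto and Micro and toggles the question widget.
; Each question is picked at random from eight, split evenly between devices, and sets hard-coded accepted ranges.
; CheckQuestion range-checks time and power, plus frequency for Magneto, and shows another question only on a correct answer.
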(event EventBeginPlay)

(event Collision|EventActorBeginOverlap
  (params (OtherActor :type Actor%20Object%20Reference)))

(event EventTick
  (params (DeltaSeconds :type Float%20%28single-precision%29)))

(fn ConstructionScript)

(fn StartExam
  (Default|StartExam (Variables|Default|Getruss))
  (Default|StartExam (Variables|Default|Getmagneto))
  (Default|StartExam (Variables|Default|Getmicro))
  (CallFunction|ShowQuestion)
  (Rendering|SetVisibility (Variables|Default|GetWidget) true false))

(fn FinishExam
  (Default|FinishExam (Variables|Default|Getruss))
  (Default|FinishExam (Variables|Default|Getmagneto))
  (Default|FinishExam (Variables|Default|Getmicro))
  (Rendering|SetVisibility (Variables|Default|GetWidget) false false))

(fn CheckQuestion
  (params (solutionPower :type Float%20%28double-precision%29) (solutionFrec :type Float%20%28double-precision%29))
  (bind _solutiontime (Variables|Default|GetsolutionTime))
  (if (Variables|Default|GetisExam)
    (LocalVariables|Setsolution_power solutionPower)
    (LocalVariables|Setsolution_frec solutionFrec)
    (if (and (<= _solutiontime (Variables|Default|GetupperTime)) (>= _solutiontime (Variables|Default|GetlowerTime)))
      (if (and (<= (LocalVariables|Getsolution_power) (Variables|Default|GetupperPower)) (>= (LocalVariables|Getsolution_power) (Variables|Default|GetlowerPower)))
        (if (Variables|Default|GetisMagneto)
          (if (and (<= (LocalVariables|Getsolution_frec) (Variables|Default|GetupperFrec)) (>= (LocalVariables|Getsolution_frec) (Variables|Default|GetlowerFrec)))
            (CallFunction|ShowQuestion :!label _label) ; Good response, next question
          )
          (else
            (goto _label)))))))

(fn ShowQuestion
  (bind _output_get (Variables|Default|SetQuestionIndex (Math|Random|RandomInteger 8)))
  (if (> _output_get 3)
    (CallFunction|SetMagnetoSolutions)
    (Variables|Default|SetisMagneto true)
    (else
      (CallFunction|SetMicroSolutions)
      (Variables|Default|SetisMagneto false)))
  (bind _asexam (Utilities|Casting|CastToExam (UserInterface|GetWidget (Variables|Default|GetWidget))))
  (Default|ChangeText _asexam (Utilities|Array|Get(acopy) (Variables|Default|GetQuestions) (Variables|Default|GetQuestionIndex))))

(fn SetMagnetoSolutions
  (Variables|Default|SetupperTime 6e+01)
  (Variables|Default|SetlowerTime 15.0)
  (bind _output_get (LocalVariables|SetRealQuestion (- (Variables|Default|GetQuestionIndex) 4))) ; There are 4 questions of micro and 4 of magneto
  (switch int _output_get
    (:0
      (Variables|Default|SetlowerPower 1e+01)
      (Variables|Default|SetupperPower 5e+01)
      (Variables|Default|SetlowerFrec 5e+01)
      (Variables|Default|SetupperFrec 1e+02))
    (:1
      (Variables|Default|SetlowerPower 5e+01)
      (Variables|Default|SetupperPower 9e+01)
      (Variables|Default|SetlowerFrec 1e+01)
      (Variables|Default|SetupperFrec 2e+01))
    (:2
      (Variables|Default|SetlowerPower 1e+01)
      (Variables|Default|SetupperPower 5e+01)
      (Variables|Default|SetlowerFrec 5e+01)
      (Variables|Default|SetupperFrec 1e+02))
    (:3
      (Variables|Default|SetlowerPower 1e+01)
      (Variables|Default|SetupperPower 5e+01)
      (Variables|Default|SetlowerFrec 1e+01)
      (Variables|Default|SetupperFrec 2e+01))))

(fn SetMicroSolutions
  (switch int (Variables|Default|GetQuestionIndex)
    (:0
      (Variables|Default|SetlowerTime 29.0)
      (Variables|Default|SetupperTime 3e+01)
      (Variables|Default|SetlowerPower 3e+01)
      (Variables|Default|SetupperPower 49.0))
    (:1
      (Variables|Default|SetlowerTime 19.0)
      (Variables|Default|SetupperTime 21.0)
      (Variables|Default|SetlowerPower 5e+01)
      (Variables|Default|SetupperPower 69.0))
    (:2
      (Variables|Default|SetlowerTime 14.0)
      (Variables|Default|SetupperTime 16.0)
      (Variables|Default|SetlowerPower 7e+01)
      (Variables|Default|SetupperPower 89.0))
    (:3
      (Variables|Default|SetlowerTime 9.0)
      (Variables|Default|SetupperTime 11.0)
      (Variables|Default|SetlowerPower 9e+01)
      (Variables|Default|SetupperPower 1.1e+02))))