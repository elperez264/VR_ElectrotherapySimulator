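; Magnetotherapy machine actor that assembles the device's buttons, indicators, screen and notifications from child actors.
; On BeginPlay it casts each child and injects references: increase/decrease buttons get their Gauss, Hz or time indicator, and the screen gets all three indicators.
; OK and power buttons target the screen, which also receives the treatment manager, while screen and applicator share the notification manager.
; StartExam and FinishExam forward to that notification manager.
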(event EventBeginPlay
  (bind _mg_hz_indicator (Variables|Default|GetMG_Hz_Indicator))
  (bind _mg_time_indicator (Variables|Default|GetMG_Time_Indicator))
  (bind _pantallamagneto (Variables|Default|GetPantallaMagneto))
  (bind _mg_gauss_indicator (Variables|Default|GetMG_Gauss_Indicator))
  (bind _childactor (Variables|/Script/Engine.ChildActorComponent|GetChildActor _mg_hz_indicator))
  (bind _childactor_2 (Variables|/Script/Engine.ChildActorComponent|GetChildActor _mg_time_indicator))
  (bind _childactor_3 (Variables|/Script/Engine.ChildActorComponent|GetChildActor _pantallamagneto))
  (bind _childactor_4 (Variables|/Script/Engine.ChildActorComponent|GetChildActor _mg_gauss_indicator))
  (bind _asincrease_mg (Utilities|Casting|CastToIncreaseMG (Variables|/Script/Engine.ChildActorComponent|GetChildActor (Variables|Default|GetIncreaseGauss))))
  (Variables|/Game/AppContent/Blueprints/Magnetotherapy/IncreaseMG.IncreaseMG_C|SetIndicator _asincrease_mg _childactor_4)
  (bind _asdecrease_mg (Utilities|Casting|CastToDecreaseMG (Variables|/Script/Engine.ChildActorComponent|GetChildActor (Variables|Default|GetDecreaseGauss))))
  (Variables|/Game/AppContent/Blueprints/Magnetotherapy/DecreaseMG.DecreaseMG_C|SetIndicator _asdecrease_mg _childactor_4)
  (bind _aspantalla_magneto (Utilities|Casting|CastToPantallaMagneto (Variables|/Script/Engine.ChildActorComponent|GetChildActor (Variables|Default|GetPantallaMagneto))))
  (bind _asmg_gauss_indicator (Utilities|Casting|CastToMG_Gauss_Indicator _childactor_4))
  (Variables|/Game/AppContent/Blueprints/Magnetotherapy/PantallaMagneto.PantallaMagneto_C|SetGaussNumber _aspantalla_magneto _asmg_gauss_indicator)
  (bind _asmg_hz_indicator (Utilities|Casting|CastToMG_Hz_Indicator _childactor))
  (Variables|/Game/AppContent/Blueprints/Magnetotherapy/PantallaMagneto.PantallaMagneto_C|SetHzNumber _aspantalla_magneto _asmg_hz_indicator)
  (bind _asincrease_mg_2 (Utilities|Casting|CastToIncreaseMG (Variables|/Script/Engine.ChildActorComponent|GetChildActor (Variables|Default|GetIncreaseHz))))
  (Variables|/Game/AppContent/Blueprints/Magnetotherapy/IncreaseMG.IncreaseMG_C|SetIndicator _asincrease_mg_2 _childactor)
  (bind _asdecrease_mg_2 (Utilities|Casting|CastToDecreaseMG (Variables|/Script/Engine.ChildActorComponent|GetChildActor (Variables|Default|GetDecreaseHz))))
  (Variables|/Game/AppContent/Blueprints/Magnetotherapy/DecreaseMG.DecreaseMG_C|SetIndicator _asdecrease_mg_2 _childactor)
  (bind _asincrease_mg_3 (Utilities|Casting|CastToIncreaseMG (Variables|/Script/Engine.ChildActorComponent|GetChildActor (Variables|Default|GetIncreaseTime))))
  (Variables|/Game/AppContent/Blueprints/Magnetotherapy/IncreaseMG.IncreaseMG_C|SetIndicator _asincrease_mg_3 _childactor_2)
  (bind _asdecrease_mg_3 (Utilities|Casting|CastToDecreaseMG (Variables|/Script/Engine.ChildActorComponent|GetChildActor (Variables|Default|GetDecreaseTime))))
  (Variables|/Game/AppContent/Blueprints/Magnetotherapy/DecreaseMG.DecreaseMG_C|SetIndicator _asdecrease_mg_3 _childactor_2)
  (bind _aspantalla_magneto_2 (Utilities|Casting|CastToPantallaMagneto (Variables|/Script/Engine.ChildActorComponent|GetChildActor (Variables|Default|GetPantallaMagneto))))
  (bind _asmg_time_indicator (Utilities|Casting|CastToMG_Time_Indicator _childactor_2))
  (Variables|/Game/AppContent/Blueprints/Magnetotherapy/PantallaMagneto.PantallaMagneto_C|SetTimeNumber _aspantalla_magneto_2 _asmg_time_indicator)
  (Variables|/Game/AppContent/Blueprints/Magnetotherapy/MG_Time_Indicator.MG_Time_Indicator_C|SetPantalla _asmg_time_indicator _aspantalla_magneto_2)
  (bind _asnotification_manager (Utilities|Casting|CastToNotificationManager (Variables|/Script/Engine.ChildActorComponent|GetChildActor (Variables|Default|GetNotificationManager))))
  (Variables|/Game/AppContent/Blueprints/Magnetotherapy/MagnetoAplicator/Magneto_Aplicator.Magneto_Aplicator_C|SetNotifications (Variables|Default|GetAplicator) _asnotification_manager)
  (Variables|/Game/AppContent/Blueprints/Magnetotherapy/PantallaMagneto.PantallaMagneto_C|SetNotifications _aspantalla_magneto_2 _asnotification_manager)
  (bind _asok_button (Utilities|Casting|CastTookButton (Variables|/Script/Engine.ChildActorComponent|GetChildActor (Variables|Default|GetokButton))))
  (Variables|/Game/AppContent/Blueprints/okButton.okButton_C|SetPantalla_Menu _asok_button _childactor_3)
  (bind _ason_off_button (Utilities|Casting|CastToOnOffButton (Variables|/Script/Engine.ChildActorComponent|GetChildActor (Variables|Default|GetOnOffButton))))
  (Variables|/Game/AppContent/Blueprints/OnOffButton.OnOffButton_C|Setpantalla _ason_off_button _childactor_3)
  (bind _aspantalla_magneto_3 (Utilities|Casting|CastToPantallaMagneto _childactor_3))
  (Variables|/Game/AppContent/Blueprints/Magnetotherapy/PantallaMagneto.PantallaMagneto_C|SetTreatmentManager _aspantalla_magneto_3 (Variables|Default|GetTreatmentManager)))

(event Collision|EventActorBeginOverlap
  (params (OtherActor :type Actor%20Object%20Reference)))

(event EventTick
  (params (DeltaSeconds :type Float%20%28single-precision%29)))

(fn ConstructionScript)

(fn StartExam
  (bind _asnotification_manager (Utilities|Casting|CastToNotificationManager (Variables|/Script/Engine.ChildActorComponent|GetChildActor (Variables|Default|GetNotificationManager))))
  (Default|StartExam _asnotification_manager))

(fn FinishExam
  (bind _asnotification_manager (Utilities|Casting|CastToNotificationManager (Variables|/Script/Engine.ChildActorComponent|GetChildActor (Variables|Default|GetNotificationManager))))
  (Default|FinishExam _asnotification_manager))