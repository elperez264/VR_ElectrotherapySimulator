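; Screen Blueprint for a magnetotherapy machine, handling power on/off and the start/pause of a timed session.
; Power events propagate to the Gauss, Hz and time number displays and toggle the off-screen overlay, with power-off also stopping the timer.
; Enter checks the minimum time and asks Notifications to approve the start, then runs a looping one-second TimeDown timer on TimeNumber.
; Countdown state is mirrored to all three displays.
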(event EventBeginPlay)

(event Collision|EventActorBeginOverlap
  (params (OtherActor :type Actor%20Object%20Reference)))

(event EventTick
  (params (DeltaSeconds :type Float%20%28single-precision%29)))

(event EventEnter
  (bind _notifications (Variables|Default|GetNotifications))
  ;[0.0625 0.0625 0.0625] If it is off the machine do nothing
  (if (Variables|Default|GetisOn)
    (if (Variables|Default|GetisCountingDown)
      ;[0.0625 0.0625 0.0625] If it is already running then pause it
      (CallFunction|FinishTimer)
      (CallFunction|NotificateCountingDown false)
      (else
        ;[0.0625 0.0625 0.0625] Check that is a valid time
        (bind _yes (Default|IsLessThanMin (Variables|Default|GetTimeNumber)))
        (if (not _yes)
          ;[0.0625 0.0625 0.0625] Notificate if it is done ok or not
          (bind _output_get (Variables|Default|SetisCountingDown true))
          (Default|SetCountingDown _notifications _output_get)
          (bind _goodstart (Default|Empezar _notifications))
          ;[0.0625 0.0625 0.0625] If it is ok then start the timer, else wait
          (if _goodstart
            (bind _returnvalue (Utilities|Time|SetTimerbyFunctionName (Variables|Default|GetTimeNumber) "TimeDown" 1.0 true))
            (bind _output_get_2 (Variables|Default|SetTimer _returnvalue))
            (Variables|/Game/AppContent/Blueprints/Magnetotherapy/MG_Time_Indicator.MG_Time_Indicator_C|SetTimer (Variables|Default|GetTimeNumber) _output_get_2)
            (bind _output_get_3 (Variables|/Game/AppContent/Blueprints/Magnetotherapy/MG_Hz_Indicator.MG_Hz_Indicator_C|SetisCountingDown (Variables|Default|GetHzNumber) true))
            (Variables|/Game/AppContent/Blueprints/Magnetotherapy/MG_Gauss_Indicator.MG_Gauss_Indicator_C|SetisCountingDown (Variables|Default|GetGaussNumber) _output_get_3)
            (else
              (bind _output_get_4 (Variables|Default|SetisCountingDown false))
              (Default|SetCountingDown (Variables|Default|GetNotifications) _output_get_4))))))))

(event EventPowerOff
  ;[0.0625 0.0625 0.0625] Reset all the number to its default value
  (Default|PowerOff (Variables|Default|GetGaussNumber))
  (Default|PowerOff (Variables|Default|GetHzNumber))
  (Default|PowerOff (Variables|Default|GetTimeNumber))
  ;[0.0625 0.0625 0.0625] The screen go off or on
  (Rendering|SetVisibility (Variables|Default|GetApagada) true false)
  (Variables|Default|SetisOn false)
  ;[0.0625 0.0625 0.0625] Stop the timer
  (CallFunction|FinishTimer)
  (CallFunction|NotificateCountingDown false))

(event EventPoweron
  (Default|Poweron (Variables|Default|GetGaussNumber))
  (Default|Poweron (Variables|Default|GetHzNumber))
  (Default|Poweron (Variables|Default|GetTimeNumber))
  ;[0.0625 0.0625 0.0625] The screen go off or on
  (Rendering|SetVisibility (Variables|Default|GetApagada) false false)
  (Variables|Default|SetisOn true))

(fn ConstructionScript)

(fn FinishTimer
  (bind _output_get (Variables|Default|SetisCountingDown false))
  (Default|SetCountingDown (Variables|Default|GetNotifications) _output_get)
  (Utilities|Time|ClearandInvalidateTimerbyHandle (Variables|Default|GetTimer))
  (CallFunction|NotificateCountingDown false))

(fn NotificateCountingDown
  (params (isCountingDown :type Boolean))
  (bind _output_get (Variables|Default|SetisCountingDown isCountingDown))
  (bind _output_get_2 (Variables|/Game/AppContent/Blueprints/Magnetotherapy/MG_Time_Indicator.MG_Time_Indicator_C|SetCountingDown (Variables|Default|GetTimeNumber) _output_get))
  (bind _output_get_3 (Variables|/Game/AppContent/Blueprints/Magnetotherapy/MG_Hz_Indicator.MG_Hz_Indicator_C|SetisCountingDown (Variables|Default|GetHzNumber) _output_get_2))
  (Variables|/Game/AppContent/Blueprints/Magnetotherapy/MG_Gauss_Indicator.MG_Gauss_Indicator_C|SetisCountingDown (Variables|Default|GetGaussNumber) _output_get_3))