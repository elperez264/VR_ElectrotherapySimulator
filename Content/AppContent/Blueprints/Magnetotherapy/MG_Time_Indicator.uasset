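; Actor for the time display of a magnetotherapy device, showing a duration in seconds on a TimeNumber widget component as minutes and seconds.
; While powered on and not counting down, Increase and Decrease step the value by five seconds within min and max limits.
; TimeDown removes one second per external call, flags counting, and calls FinishTimer on Pantalla at zero.
; PowerOff resets to the minimum.
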(event EventBeginPlay)

(event Collision|EventActorBeginOverlap
  (params (OtherActor :type Actor%20Object%20Reference)))

(event EventTick
  (params (DeltaSeconds :type Float%20%28single-precision%29)))

(event EventPowerOff
  (Variables|Default|SetValueSeconds (Variables|Default|GetMinValue))
  (bind _astime_number (Utilities|Casting|CastToTimeNumber (UserInterface|GetUserWidgetObject (Variables|Default|GetWidget))))
  (Default|SetValueEvent _astime_number (/ (Variables|Default|GetValueSeconds) 60) (Math|Integer|%(Integer) (Variables|Default|GetValueSeconds) 60))
  (Variables|Default|SetisOn false))

(event EventDecrease
  (if (and (Variables|Default|GetisOn) (not (Variables|Default|GetCountingDown)))
    (bind _yes (CallFunction|IsMin))
    (if (not _yes)
      (CallFunction|DecreaseTime 5))))

(event EventIncrease
  (if (and (Variables|Default|GetisOn) (not (Variables|Default|GetCountingDown)))
    (bind _yes (CallFunction|IsMax))
    (if (not _yes)
      (bind _output_get (Variables|Default|SetValueSeconds (+ (Variables|Default|GetValueSeconds) 5)))
      (bind _astime_number (Utilities|Casting|CastToTimeNumber (UserInterface|GetUserWidgetObject (Variables|Default|GetWidget))))
      (Default|SetValueEvent _astime_number (/ _output_get 60) (Math|Integer|%(Integer) _output_get 60)))))

(fn ConstructionScript)

(fn TimeDown
  (if (>= (Variables|Default|GetValueSeconds) 1)
    (CallFunction|DecreaseTime 1)
    (Variables|Default|SetCountingDown true)
    (else
      (Default|FinishTimer (Variables|Default|GetPantalla))
      (Variables|Default|SetCountingDown false))))

(fn DecreaseTime
  (params (Delta :type Integer))
  (bind _output_get (Variables|Default|SetValueSeconds (- (Variables|Default|GetValueSeconds) Delta)))
  (bind _astime_number (Utilities|Casting|CastToTimeNumber (UserInterface|GetUserWidgetObject (Variables|Default|GetWidget))))
  (Default|SetValueEvent _astime_number (/ _output_get 60) (Math|Integer|%(Integer) _output_get 60)))

(fn IsLessThanMin
  (return (< (Variables|Default|GetValueSeconds) (Variables|Default|GetMinValue))))

(fn Poweron
  (Variables|Default|SetisOn true))

(fn IsMax
  (return (>= (Variables|Default|GetValueSeconds) (Variables|Default|GetMaxValue))))

(fn IsMin
  (return (<= (Variables|Default|GetValueSeconds) (Variables|Default|GetMinValue))))