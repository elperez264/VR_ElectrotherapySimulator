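; VRButton is a physical push button that VR pawns trigger by touch.
; Tick polls the ButtonCollision volume for overlapping VRPawn actors instead of using overlap events.
; A detection lowers the Cube by MovingOffset, calls Press, then raises it again.
; The IsMoving flag and a short delay block re-entry, so the press repeats while the pawn stays inside.
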(event EventBeginPlay)

(event Collision|EventActorBeginOverlap
  (params (OtherActor :type Actor%20Object%20Reference)))

(event EventTick
  (params (DeltaSeconds :type Float%20%28single-precision%29))
  (bind _cube (Variables|Default|GetCube))
  (bind _cube_2 (Variables|Default|GetCube))
  (if (> (Utilities|Array|Length (Collision|GetOverlappingActors (Variables|Default|GetButtonCollision) "/Game/VRTemplate/Blueprints/VRPawn.VRPawn_C" :!class /Script/Engine.PrimitiveComponent)) 0)
    (if (not (Variables|Default|GetIsMoving))
      (Variables|Default|SetIsMoving true)
      (Components|MoveComponentTo _cube (Math|Vector|MakeVector 0.0 0.0 (- (.z (Variables|/Script/Engine.SceneComponent|GetRelativeLocation _cube)) (Variables|Default|GetMovingOffset))) (Variables|/Script/Engine.SceneComponent|GetRelativeRotation _cube) false false 0.1 false)
      (CallFunction|Press)
      (Components|MoveComponentTo _cube_2 (Math|Vector|MakeVector 0.0 0.0 (+ (.z (Variables|/Script/Engine.SceneComponent|GetRelativeLocation _cube_2)) (Variables|Default|GetMovingOffset))) (Variables|/Script/Engine.SceneComponent|GetRelativeRotation _cube_2) false false 0.1 false)
      (Utilities|FlowControl|Delay 0.2)
      (Variables|Default|SetIsMoving false))))

(fn ConstructionScript)