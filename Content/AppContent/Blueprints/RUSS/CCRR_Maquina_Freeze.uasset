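; CCRR_Maquina_Freeze is a machine actor assembled from child actors: a PantallaCorrientes screen, a NotificationManager and a panel of buttons.
; On BeginPlay it casts and caches each child actor, then hands the notification manager to the screen.
; It then gives the up, down, plus, minus, on/off and OK buttons a reference to that screen.
; The actor itself only does this wiring.
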(event EventBeginPlay
  ;[0.0625 0.0625 0.0625] Cast every variable to its class
  (CallFunction|InitializeVariables)
  (CallFunction|InitializeScreen)
  (CallFunction|InitializeUpButton)
  (CallFunction|InitializeDownButton)
  (CallFunction|Initialize+Button)
  (CallFunction|Initialize-Button)
  (CallFunction|InitializeonOffButton)
  (CallFunction|InitializeOkButton))

(event Collision|EventActorBeginOverlap
  (params (OtherActor :type Actor%20Object%20Reference)))

(event EventTick
  (params (DeltaSeconds :type Float%20%28single-precision%29)))

(fn ConstructionScript)

(fn InitializeVariables
  (bind _asgo_down (Utilities|Casting|CastToGoDown (Variables|/Script/Engine.ChildActorComponent|GetChildActor (Variables|Default|GetGoDown))))
  (Variables|Default|SetAs%20Go%20Down _asgo_down)
  (bind _as__button (Utilities|Casting|CastTo-Button (Variables|/Script/Engine.ChildActorComponent|GetChildActor (Variables|Default|Get-Button))))
  (Variables|Default|SetAs-%20Button _as__button)
  (bind _as__button_2 (Utilities|Casting|CastTo+Button (Variables|/Script/Engine.ChildActorComponent|GetChildActor (Variables|Default|Get+Button))))
  (Variables|Default|SetAs+%20Button _as__button_2)
  (bind _asgo_up (Utilities|Casting|CastToGoUp (Variables|/Script/Engine.ChildActorComponent|GetChildActor (Variables|Default|GetGoUp))))
  (Variables|Default|SetAs%20Go%20Up _asgo_up)
  (bind _asnotification_manager (Utilities|Casting|CastToNotificationManager (Variables|/Script/Engine.ChildActorComponent|GetChildActor (Variables|Default|GetNotificationManager))))
  (Variables|Default|SetAs%20Notification%20Manager _asnotification_manager)
  (bind _asok_button (Utilities|Casting|CastTookButton (Variables|/Script/Engine.ChildActorComponent|GetChildActor (Variables|Default|GetokButton))))
  (Variables|Default|SetAs%20Ok%20Button _asok_button)
  (bind _aspantalla_corrientes (Utilities|Casting|CastToPantallaCorrientes (Variables|/Script/Engine.ChildActorComponent|GetChildActor (Variables|Default|GetPantallaCorrientes))))
  (Variables|Default|SetAs%20Pantalla%20Corrientes _aspantalla_corrientes)
  (bind _ason_off_button (Utilities|Casting|CastToOnOffButton (Variables|/Script/Engine.ChildActorComponent|GetChildActor (Variables|Default|GetOnOffButton))))
  (Variables|Default|SetAs%20on%20Off%20Button _ason_off_button))

(fn InitializeScreen
  (Variables|/Game/AppContent/Blueprints/RUSS/PantallaCorrientes.PantallaCorrientes_C|SetNotifications (Variables|Default|GetAs%20Pantalla%20Corrientes) (Variables|Default|GetAs%20Notification%20Manager)))

(fn InitializeUpButton
  (Variables|/Game/AppContent/Blueprints/RUSS/GoUp.GoUp_C|SetPantalla (Variables|Default|GetAs%20Go%20Up) (Variables|Default|GetAs%20Pantalla%20Corrientes)))

(fn InitializeDownButton
  (Variables|/Game/AppContent/Blueprints/RUSS/GoDown.GoDown_C|SetPantalla (Variables|Default|GetAs%20Go%20Down) (Variables|Default|GetAs%20Pantalla%20Corrientes)))

(fn Initialize+Button
  (Variables|/Game/AppContent/Blueprints/RUSS/+Button.+Button_C|SetPantalla (Variables|Default|GetAs+%20Button) (Variables|Default|GetAs%20Pantalla%20Corrientes)))

(fn Initialize-Button
  (Variables|/Game/AppContent/Blueprints/RUSS/-Button.-Button_C|SetPantalla (Variables|Default|GetAs-%20Button) (Variables|Default|GetAs%20Pantalla%20Corrientes)))

(fn InitializeonOffButton
  (Variables|/Game/AppContent/Blueprints/OnOffButton.OnOffButton_C|Setpantalla (Variables|Default|GetAs%20on%20Off%20Button) (Variables|Default|GetAs%20Pantalla%20Corrientes)))

(fn InitializeOkButton
  (Variables|/Game/AppContent/Blueprints/okButton.okButton_C|SetPantalla_Menu (Variables|Default|GetAs%20Ok%20Button) (Variables|Default|GetAs%20Pantalla%20Corrientes)))