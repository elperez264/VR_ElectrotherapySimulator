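; Control screen of a RUSS electrotherapy device for choosing body part, method, time, pulse, pause and two intensities.
; A seven-row menu moves a highlight and routes next/previous input to setters that update a child numeric indicator.
; Enter toggles a one-second countdown after TreatmentManager, Patient and Notifications checks.
; At start, Intensity1 is graded against a range to set the patient's NPC reaction power; PowerOff resets everything.
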(event EventBeginPlay
  (Variables|Default|SetActualMenu (Variables|Default|GetBodyPart))
  (bind _asruss_numbers_indicator (Utilities|Casting|CastToRUSS_Numbers_Indicator (Variables|/Script/Engine.ChildActorComponent|GetChildActor (Variables|Default|GetRUSS_Numbers_Indicator))))
  (Default|SetMaxPause _asruss_numbers_indicator 6e+01)
  (Default|SetMaxPulse _asruss_numbers_indicator 6e+01))

(event Collision|EventActorBeginOverlap
  (params (OtherActor :type Actor%20Object%20Reference)))

(event EventTick
  (params (DeltaSeconds :type Float%20%28single-precision%29)))

(event EventEnter
  (bind _patient (Variables|Default|GetPatient))
  (bind _notifications (Variables|Default|GetNotifications))
  (if (Variables|Default|GetisOn)
    ;[0.04167 0.04167 0.04167] If the timer is setted then stop it, if not, start it
    (if (Variables|Default|GetisCountingDown)
      (bind _output_get (Variables|Default|SetisCountingDown false))
      (Default|SetCountingDown (Variables|Default|GetNotifications) _output_get)
      (Utilities|Time|ClearandInvalidateTimerbyHandle (Variables|Default|GetTimer))
      (Default|StopTreatment (Variables|Default|GetTreatmentManager))
      (Default|StopAplication (Variables|Default|GetPatient))
      (elif (> (Variables|Default|GetTimeValueSeconds) 0)
        (bind _treatmentstarting (Default|StartTreatment (Variables|Default|GetTreatmentManager)))
        (if _treatmentstarting
          ;[0.04688 0.04688 0.04688] Set the manager of the aplicator to start the process
          (Default|SetManager (Variables|Default|GetAplicator) (Variables|Default|GetNotifications))
          (Variables|/Game/AppContent/Blueprints/NPC/NPC.NPC_C|SetPower _patient 0.0)
          (bind _aplicated (Default|CheckAplications _patient))
          (if _aplicated
            ;[0.0625 0.0625 0.0625] Notificate if it is ok or not
            (bind _output_get_2 (Variables|Default|SetisCountingDown true))
            (Default|SetCountingDown _notifications _output_get_2)
            (bind _goodstart (Default|Empezar _notifications))
            (if _goodstart
              ;[0.0625 0.0625 0.0625] If everything is ok start, else wait
              (bind _returnvalue (Utilities|Time|SetTimerbyFunctionName 0 "DecreaseOneSecond" 1.0 true))
              (Variables|Default|SetTimer _returnvalue)
              (bind _good_start (CallFunction|ComunicationNPC))
              (if _good_start
                _)
              (else
                (bind _output_get_3 (Variables|Default|SetisCountingDown false))
                (Default|SetCountingDown (Variables|Default|GetNotifications) _output_get_3)
                (Default|StopTreatment (Variables|Default|GetTreatmentManager))
                (Default|StopAplication (Variables|Default|GetPatient))))
            (else
              (Default|StopTreatment (Variables|Default|GetTreatmentManager))))
          (else
            (Default|AlreadyRunning (Variables|Default|GetNotifications))))))))

(event EventPowerOff
  (bind _notifications (Variables|Default|GetNotifications))
  (Rendering|SetVisibility (Variables|Default|GetPantallaApagada) true false)
  (if (Variables|Default|GetisCountingDown)
    ;[0.04167 0.04167 0.04167] Stop de timer and tell the notification that is off
    (Utilities|Time|ClearandInvalidateTimerbyHandle (Variables|Default|GetTimer))
    (bind _output_get (Variables|Default|SetisCountingDown false))
    (Default|SetCountingDown _notifications _output_get)
    ;[0.04167 0.04167 0.04167] Is counting down when the button off is pressed
    (Default|Apagar _notifications true))
  ;[0.04167 0.04167 0.04167] Reset all the values and menu to the default value
  (CallFunction|ResetMenu)
  (CallFunction|ResetMethod)
  (CallFunction|ResetBodyPart)
  (CallFunction|ResetTimes)
  (Variables|Default|SetisOn false)
  (Default|StopTreatment (Variables|Default|GetTreatmentManager))
  (Default|StopAplication (Variables|Default|GetPatient)))

(event EventPoweron
  (Rendering|SetVisibility (Variables|Default|GetPantallaApagada) false false)
  (Variables|Default|SetisOn true))

(fn ConstructionScript
  (bind _output_get (Variables|Default|SetSelectionPosition (Variables|/Script/Engine.SceneComponent|GetRelativeLocation (Variables|Default|GetMenuSelection))))
  (Variables|Default|SetInitialPosition _output_get))

(fn NextonSelection
  (if (Variables|Default|GetisOn)
    (switch int (Variables|Default|GetIndiceMenu)
      (:0
        (CallFunction|NextPart))
      (:1
        (CallFunction|NextMethod))
      (:2
        (if (not (Variables|Default|GetisCountingDown))
          (CallFunction|IncreaseTime)))
      (:3
        (if (not (Variables|Default|GetisCountingDown))
          (CallFunction|IncreasePulse)))
      (:4
        (if (not (Variables|Default|GetisCountingDown))
          (CallFunction|IncreasePause)))
      (:5
        (if (not (Variables|Default|GetisCountingDown))
          (CallFunction|IncreaseIntensity1)))
      (:6
        (if (not (Variables|Default|GetisCountingDown))
          (CallFunction|IncreaseIntensity2))))))

(fn PreviousonSelection
  (if (Variables|Default|GetisOn)
    (switch int (Variables|Default|GetIndiceMenu)
      (:0
        (CallFunction|PreviousPart))
      (:1
        (CallFunction|PreviousMethod))
      (:2
        (if (not (Variables|Default|GetisCountingDown))
          (CallFunction|DecreaseTime)))
      (:3
        (if (not (Variables|Default|GetisCountingDown))
          (CallFunction|DecreasePulse)))
      (:4
        (if (not (Variables|Default|GetisCountingDown))
          (CallFunction|DecreasePause)))
      (:5
        (if (not (Variables|Default|GetisCountingDown))
          (CallFunction|DecreaseIntensity1)))
      (:6
        (if (not (Variables|Default|GetisCountingDown))
          (CallFunction|DecreaseIntensity2))))))

(fn NextMenu
  (if (Variables|Default|GetisOn)
    (if (not (> (Variables|Default|GetIndiceMenu) 5))
      (Transformation|SetRelativeLocation (Variables|Default|GetMenuSelection) (Math|Vector|MakeVector (.x (Variables|Default|GetSelectionPosition)) (+ (.y (Variables|Default|GetSelectionPosition)) 12.0) (.z (Variables|Default|GetSelectionPosition))) false false)
      (Variables|Default|SetSelectionPosition (Math|Vector|MakeVector (.x (Variables|Default|GetSelectionPosition)) (+ (.y (Variables|Default|GetSelectionPosition)) 12.0) (.z (Variables|Default|GetSelectionPosition))))
      (Variables|Default|SetIndiceMenu (+ (Variables|Default|GetIndiceMenu) 1))
      (CallFunction|ChangeActualMenu)
      (CallFunction|ChangeColor (Variables|Default|GetPrevious%20Menu) (Variables|Default|GetActualMenu)))))

(fn PreviousMenu
  (if (Variables|Default|GetisOn)
    (if (not (< (Variables|Default|GetIndiceMenu) 1))
      (Transformation|SetRelativeLocation (Variables|Default|GetMenuSelection) (Math|Vector|MakeVector (.x (Variables|Default|GetSelectionPosition)) (+ (.y (Variables|Default|GetSelectionPosition)) -12.0) (.z (Variables|Default|GetSelectionPosition))) false false)
      (Variables|Default|SetSelectionPosition (Math|Vector|MakeVector (.x (Variables|Default|GetSelectionPosition)) (+ (.y (Variables|Default|GetSelectionPosition)) -12.0) (.z (Variables|Default|GetSelectionPosition))))
      (Variables|Default|SetIndiceMenu (+ (Variables|Default|GetIndiceMenu) -1))
      (CallFunction|ChangeActualMenu)
      (CallFunction|ChangeColor (Variables|Default|GetPrevious%20Menu) (Variables|Default|GetActualMenu)))))

(fn ChangeActualMenu
  ;[0.04167 0.04167 0.04167] Set the text of the actual menu and set the previous menu
  (Variables|Default|SetPrevious%20Menu (Variables|Default|GetActualMenu))
  (switch int (Variables|Default|GetIndiceMenu)
    (:0
      (Variables|Default|SetActualMenu (Variables|Default|GetBodyPart)))
    (:1
      (Variables|Default|SetActualMenu (Variables|Default|GetMethod))
      (Rendering|Material|SetMaterial (Variables|Default|GetImage) 0 (Variables|Default|GetActualImage))
      (Rendering|SetVisibility (Variables|Default|GetRUSS_Numbers_Indicator) false false))
    (:2
      (Variables|Default|SetActualMenu (Variables|Default|GetTime))
      (Rendering|Material|SetMaterial (Variables|Default|GetImage) 0 "/Engine/BasicShapes/BasicShapeMaterial.BasicShapeMaterial")
      (Rendering|SetVisibility (Variables|Default|GetRUSS_Numbers_Indicator) true false))
    (:3
      (Variables|Default|SetActualMenu (Variables|Default|GetImpulso)))
    (:4
      (Variables|Default|SetActualMenu (Variables|Default|GetPausa)))
    (:5
      (Variables|Default|SetActualMenu (Variables|Default|GetIntensidad%201)))
    (:6
      (Variables|Default|SetActualMenu (Variables|Default|GetIntensidad%202)))))

(fn ChangeColor
  (params (Previous :type Text%20Render%20Component%20Object%20Reference) (Next :type Text%20Render%20Component%20Object%20Reference))
  ;[0.04167 0.04167 0.04167] Set black
  (Rendering|Components|TextRender|SetTextRenderColor Previous (Math|Color|MakeColor 0 0 0 0))
  ;[0.04167 0.04167 0.04167] Set white
  (Rendering|Components|TextRender|SetTextRenderColor Next (Math|Color|MakeColor 255 255 255 255)))

(fn NextPart
  (if (<= (+ (Variables|Default|GetIndiceParts) 1) 5)
    (bind _output_get (Variables|Default|SetIndiceParts (+ (Variables|Default|GetIndiceParts) 1)))
    (Rendering|Components|TextRender|SetText (Variables|Default|GetBodyIndicator) (Utilities|Array|Get(acopy) (Variables|Default|GetBodyParts) _output_get))
    (CallFunction|ChangeImage (Utilities|Array|Get(acopy) (Variables|Default|GetBodyParts) _output_get))))

(fn PreviousPart
  (if (>= (+ (Variables|Default|GetIndiceParts) -1) 0)
    (bind _output_get (Variables|Default|SetIndiceParts (+ (Variables|Default|GetIndiceParts) -1)))
    (Rendering|Components|TextRender|SetText (Variables|Default|GetBodyIndicator) (Utilities|Array|Get(acopy) (Variables|Default|GetBodyParts) _output_get))
    (CallFunction|ChangeImage (Utilities|Array|Get(acopy) (Variables|Default|GetBodyParts) _output_get))))

(fn NextMethod
  (if (<= (+ (Variables|Default|GetIndiceMethods) 1) 1)
    (bind _output_get (Variables|Default|SetIndiceMethods (+ (Variables|Default|GetIndiceMethods) 1)))
    (Rendering|Components|TextRender|SetText (Variables|Default|GetMethodIndicator) (Utilities|Array|Get(acopy) (Variables|Default|GetMethods) _output_get))))

(fn PreviousMethod
  (if (>= (+ (Variables|Default|GetIndiceMethods) -1) 0)
    (bind _output_get (Variables|Default|SetIndiceMethods (+ (Variables|Default|GetIndiceMethods) -1)))
    (Rendering|Components|TextRender|SetText (Variables|Default|GetMethodIndicator) (Utilities|Array|Get(acopy) (Variables|Default|GetMethods) _output_get))))

(fn ChangeActualMaterial
  (params (Name :type Text))
  (switch string (Utilities|String|ToString(Text) Name)
    (:Hand
      (Variables|Default|SetActualImage "/Game/AppContent/Materials/HandTexture.HandTexture"))
    (:Neck
      (Variables|Default|SetActualImage "/Game/AppContent/Materials/NeckTexture.NeckTexture"))
    (:Shoulders
      (Variables|Default|SetActualImage "/Game/AppContent/Materials/ShouldersTexture.ShouldersTexture"))
    (:Back
      (Variables|Default|SetActualImage "/Game/AppContent/Materials/BackTexture.BackTexture"))
    (:Feet
      (Variables|Default|SetActualImage "/Game/AppContent/Materials/FeetTexture.FeetTexture"))
    (:Legs
      (Variables|Default|SetActualImage "/Game/AppContent/Materials/LegsTexture.LegsTexture"))))

(fn ChangeImage
  (params (Name :type Text))
  (CallFunction|ChangeActualMaterial Name)
  (Rendering|Material|SetMaterial (Variables|Default|GetImage) 0 (Variables|Default|GetActualImage)))

(fn IncreasePulse
  (if (< (+ (Variables|Default|GetPulseValue) 1) 61)
    (Variables|Default|SetPulseValue (+ (Variables|Default|GetPulseValue) 1))
    (bind _asruss_numbers_indicator (Utilities|Casting|CastToRUSS_Numbers_Indicator (Variables|/Script/Engine.ChildActorComponent|GetChildActor (Variables|Default|GetRUSS_Numbers_Indicator))))
    (Default|ChangePulse _asruss_numbers_indicator (Variables|Default|GetPulseValue))))

(fn DecreasePulse
  (if (> (+ (Variables|Default|GetPulseValue) -1) 0)
    (Variables|Default|SetPulseValue (+ (Variables|Default|GetPulseValue) -1))
    (bind _asruss_numbers_indicator (Utilities|Casting|CastToRUSS_Numbers_Indicator (Variables|/Script/Engine.ChildActorComponent|GetChildActor (Variables|Default|GetRUSS_Numbers_Indicator))))
    (Default|ChangePulse _asruss_numbers_indicator (Variables|Default|GetPulseValue))))

(fn IncreasePause
  (if (< (+ (Variables|Default|GetPauseValue) 1) 61)
    (Variables|Default|SetPauseValue (+ (Variables|Default|GetPauseValue) 1))
    (bind _asruss_numbers_indicator (Utilities|Casting|CastToRUSS_Numbers_Indicator (Variables|/Script/Engine.ChildActorComponent|GetChildActor (Variables|Default|GetRUSS_Numbers_Indicator))))
    (Default|ChangePause _asruss_numbers_indicator (Variables|Default|GetPauseValue))))

(fn DecreasePause
  (if (> (+ (Variables|Default|GetPauseValue) -1) 4)
    (Variables|Default|SetPauseValue (+ (Variables|Default|GetPauseValue) -1))
    (bind _asruss_numbers_indicator (Utilities|Casting|CastToRUSS_Numbers_Indicator (Variables|/Script/Engine.ChildActorComponent|GetChildActor (Variables|Default|GetRUSS_Numbers_Indicator))))
    (Default|ChangePause _asruss_numbers_indicator (Variables|Default|GetPauseValue))))

(fn IncreaseTime
  (if (< (+ (Variables|Default|GetTimeValueSeconds) 300) 3601)
    (Variables|Default|SetTimeValueSeconds (+ (Variables|Default|GetTimeValueSeconds) 300))
    (bind _asruss_numbers_indicator (Utilities|Casting|CastToRUSS_Numbers_Indicator (Variables|/Script/Engine.ChildActorComponent|GetChildActor (Variables|Default|GetRUSS_Numbers_Indicator))))
    (Default|ChangeTime _asruss_numbers_indicator (Variables|Default|GetTimeValueSeconds))))

(fn DecreaseTime
  (if (> (+ (Variables|Default|GetTimeValueSeconds) -300) 299)
    (Variables|Default|SetTimeValueSeconds (+ (Variables|Default|GetTimeValueSeconds) -300))
    (else
      (Variables|Default|SetTimeValueSeconds 300)))
  (bind _asruss_numbers_indicator (Utilities|Casting|CastToRUSS_Numbers_Indicator (Variables|/Script/Engine.ChildActorComponent|GetChildActor (Variables|Default|GetRUSS_Numbers_Indicator))))
  (Default|ChangeTime _asruss_numbers_indicator (Variables|Default|GetTimeValueSeconds)))

(fn DecreaseOneSecond
  (if (> (+ (Variables|Default|GetTimeValueSeconds) -1) -1)
    (Variables|Default|SetTimeValueSeconds (+ (Variables|Default|GetTimeValueSeconds) -1))
    (bind _asruss_numbers_indicator (Utilities|Casting|CastToRUSS_Numbers_Indicator (Variables|/Script/Engine.ChildActorComponent|GetChildActor (Variables|Default|GetRUSS_Numbers_Indicator))))
    (Default|ChangeTime _asruss_numbers_indicator (Variables|Default|GetTimeValueSeconds))
    (else
      (Variables|Default|SetisCountingDown false)
      (Utilities|Time|ClearandInvalidateTimerbyHandle (Variables|Default|GetTimer))
      (Default|StopAplication (Variables|Default|GetPatient)))))

(fn ResetMenu
  (Variables|Default|SetIndiceMenu 0)
  (CallFunction|ChangeActualMenu)
  (CallFunction|ChangeColor (Variables|Default|GetPrevious%20Menu) (Variables|Default|GetActualMenu))
  (Transformation|SetRelativeLocation (Variables|Default|GetMenuSelection) (Variables|Default|GetInitialPosition) false false)
  (Variables|Default|SetSelectionPosition (Variables|Default|GetInitialPosition)))

(fn ResetBodyPart
  (bind _output_get (Variables|Default|SetIndiceParts 0))
  (Rendering|Components|TextRender|SetText (Variables|Default|GetBodyIndicator) (Utilities|Array|Get(acopy) (Variables|Default|GetBodyParts) _output_get))
  (CallFunction|ChangeImage (Utilities|Array|Get(acopy) (Variables|Default|GetBodyParts) _output_get)))

(fn ResetMethod
  (bind _output_get (Variables|Default|SetIndiceMethods 0))
  (Rendering|Components|TextRender|SetText (Variables|Default|GetMethodIndicator) (Utilities|Array|Get(acopy) (Variables|Default|GetMethods) _output_get)))

(fn ResetTimes
  ;[0.0625 0.0625 0.0625] Reset time, pulse, pause and intensities
  (Rendering|SetVisibility (Variables|Default|GetRUSS_Numbers_Indicator) false false)
  (bind _asruss_numbers_indicator (Utilities|Casting|CastToRUSS_Numbers_Indicator (Variables|/Script/Engine.ChildActorComponent|GetChildActor (Variables|Default|GetRUSS_Numbers_Indicator))))
  (bind _output_get (Variables|Default|SetTimeValueSeconds 0))
  (Default|ChangeTime _asruss_numbers_indicator _output_get)
  (bind _output_get_2 (Variables|Default|SetPulseValue 1))
  (Default|ChangePulse _asruss_numbers_indicator _output_get_2)
  (bind _output_get_3 (Variables|Default|SetPauseValue 5))
  (Default|ChangePause _asruss_numbers_indicator _output_get_3)
  (bind _output_get_4 (Variables|Default|SetIntensity1 0.016))
  (Default|ChangeIntensity1 _asruss_numbers_indicator _output_get_4)
  (bind _output_get_5 (Variables|Default|SetIntensity2 0.016))
  (Default|ChangeIntensity2 _asruss_numbers_indicator _output_get_5))

(fn IncreaseIntensity1
  (if (< (+ (Variables|Default|GetIntensity1) 0.02) 1.02)
    (Variables|Default|SetIntensity1 (+ (Variables|Default|GetIntensity1) 0.02))
    (bind _asruss_numbers_indicator (Utilities|Casting|CastToRUSS_Numbers_Indicator (Variables|/Script/Engine.ChildActorComponent|GetChildActor (Variables|Default|GetRUSS_Numbers_Indicator))))
    (Default|ChangeIntensity1 _asruss_numbers_indicator (Variables|Default|GetIntensity1))))

(fn IncreaseIntensity2
  (if (< (+ (Variables|Default|GetIntensity2) 0.02) 1.02)
    (Variables|Default|SetIntensity2 (+ (Variables|Default|GetIntensity2) 0.02))
    (bind _asruss_numbers_indicator (Utilities|Casting|CastToRUSS_Numbers_Indicator (Variables|/Script/Engine.ChildActorComponent|GetChildActor (Variables|Default|GetRUSS_Numbers_Indicator))))
    (Default|ChangeIntensity2 _asruss_numbers_indicator (Variables|Default|GetIntensity2))))

(fn DecreaseIntensity1
  (if (> (+ (Variables|Default|GetIntensity1) -0.02) 0.0)
    (Variables|Default|SetIntensity1 (+ (Variables|Default|GetIntensity1) -0.02))
    (bind _asruss_numbers_indicator (Utilities|Casting|CastToRUSS_Numbers_Indicator (Variables|/Script/Engine.ChildActorComponent|GetChildActor (Variables|Default|GetRUSS_Numbers_Indicator))))
    (Default|ChangeIntensity1 _asruss_numbers_indicator (Variables|Default|GetIntensity1))))

(fn DecreaseIntensity2
  (if (> (+ (Variables|Default|GetIntensity2) -0.02) 0.0)
    (Variables|Default|SetIntensity2 (+ (Variables|Default|GetIntensity2) -0.02))
    (bind _asruss_numbers_indicator (Utilities|Casting|CastToRUSS_Numbers_Indicator (Variables|/Script/Engine.ChildActorComponent|GetChildActor (Variables|Default|GetRUSS_Numbers_Indicator))))
    (Default|ChangeIntensity2 _asruss_numbers_indicator (Variables|Default|GetIntensity2))))

(fn GetPower
  (params (intensity :type Float%20%28double-precision%29) (upperCup :type Float%20%28double-precision%29) (lowerCup :type Float%20%28double-precision%29))
  ;[0.04688 0.04688 0.04688] The result power is for the NPC animation, we check that the intensity is in the patient range
  (if (>= intensity lowerCup)
    (if (<= intensity upperCup)
      (return 1e+02)
      (else
        (return 2e+02)))
    (else
      (return 0.0))))

(fn ComunicationNPC
  (bind _patient (Variables|Default|GetPatient))
  (bind _finalpower (CallFunction|GetPower (Variables|Default|GetIntensity1) (Variables|Default|GetupperCup1) (Variables|Default|GetlowerCup1)))
  (Variables|/Game/AppContent/Blueprints/NPC/NPC.NPC_C|SetPower _patient _finalpower)
  (bind _goodstart (Default|StartAplication _patient))
  (return _goodstart))