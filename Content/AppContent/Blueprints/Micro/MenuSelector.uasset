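; MenuSelector is a grabbable wheel that operates the menu selector on a screen (Pantalla) when twisted by a motion controller.
; On grab, it stores the controller's relative yaw and starts a looping timer to compare against it.
; When yaw rises past a dead zone, it calls UseMenuSelector, turns the wheel by that delta and resets the reference; decreasing yaw does nothing.
; Dropping clears the controller and pauses the timer.
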(event OnGrabbed(GrabComponent)
  (params (MotionControler :type Motion%20Controller%20Component%20Object%20Reference))
  ;[0.06771 0.06771 0.06771] Set the initial rotation of the controler and start the timer while is grabbed
  (bind _output_get (Variables|Default|SetMotion%20Controler MotionControler))
  (Variables|Default|SetCurrentControlerRotation (.yaw (Variables|/Script/Engine.SceneComponent|GetRelativeRotation _output_get)))
  (Utilities|Time|SetTimerbyEvent (delegate Custom|UpdateRotation) (Variables|Default|GetTimeLap) true))

(event OnDropped(GrabComponent)
  ;[0.04167 0.04167 0.04167] Clear the motion controler and stop the timer
  (Variables|Default|SetMotion%20Controler 0)
  (Class|KismetSystemLibrary|PauseTimer 0 "UpdateRotation"))

(event Custom|UpdateRotation
  (bind _motion_controler (Variables|Default|GetMotion%20Controler))
  (bind _relativerotation (Variables|/Script/Engine.SceneComponent|GetRelativeRotation _motion_controler))
  ;[0.0625 0.0625 0.0625] control if the hand have rotate enough to the left or the right to increase or decrease the value, then rotate the wheel with the same rotation as the wheel
  (bind _output_get (Variables|Default|Setdelta (- (.yaw _relativerotation) (Variables|Default|GetCurrentControlerRotation))))
  (if (> (Math|Float|Absolute(Float) _output_get) (Variables|Default|GetrotationDeadPoint))
    (if (< (Variables|Default|GetCurrentControlerRotation) (.yaw _relativerotation))
      (CallFunction|Increase)
      (Variables|Default|SetCurrentControlerRotation (.yaw _relativerotation))
      (Transformation|AddRelativeRotation (Variables|Default|GetWheel) (Math|Rotator|MakeRotator 0.0 0.0 (Variables|Default|Getdelta)) false false))))

(event EventBeginPlay)

(event Collision|EventActorBeginOverlap
  (params (OtherActor :type Actor%20Object%20Reference)))

(event EventTick
  (params (DeltaSeconds :type Float%20%28single-precision%29)))

(event EventIncrease
  ;[0.0625 0.0625 0.0625] Rotate the wheel
  (Default|UseMenuSelector (Variables|Default|GetPantalla)))

(fn ConstructionScript)