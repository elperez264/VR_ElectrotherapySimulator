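; Two-digit countdown display for the Micro device, built from two TextRender components that show only while powered on.
; Increase and Decrease adjust the value, split into digit characters for display; increasing is blocked during countdown.
; StartTimer runs DecreaseValue every second if NotificationManager approves the start, reporting countdown state to it.
; Reaching the minimum stops the timer and notifies PantallaMenu; powering off resets the value and cancels any countdown.
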(event EventBeginPlay)

(event Collision|EventActorBeginOverlap
  (params (OtherActor :type Actor%20Object%20Reference)))

(event EventTick
  (params (DeltaSeconds :type Float%20%28single-precision%29)))

(event EventDecrease
  (CallFunction|DecreaseValue))

(event EventIncrease
  (CallFunction|IncreaseValue))

(fn ConstructionScript)

(fn IncreaseValue
  (if (and (Variables|Default|GetEncendido) (not (Variables|Default|GetCountingDown)))
    (Variables|Default|SetValue (+ 1 (Variables|Default|GetValue)))
    (bind (_first _second) (CallFunction|GetNumbers (Utilities|String|ToString(Integer) (+ 1 (Variables|Default|GetValue)))))
    (CallFunction|SetNumbers _first _second)))

(fn DecreaseValue
  (if (> (Variables|Default|GetValue) 1)
    (if (Variables|Default|GetEncendido)
      (Variables|Default|SetValue (+ -1 (Variables|Default|GetValue)))
      (bind (_first _second) (CallFunction|GetNumbers (Utilities|String|ToString(Integer) (+ -1 (Variables|Default|GetValue)))))
      (CallFunction|SetNumbers _first _second)
      (if (<= (Variables|Default|GetValue) 1)
        _))
    (else
      (CallFunction|StopTimer))))

(fn GetPower
  (return (Variables|Default|GetValue)))

(fn GetNumbers
  (params (Input :type String))
  (bind _returnvalue (Utilities|String|GetCharacterArrayfromString Input))
  (bind _output (Utilities|Array|Get(acopy) _returnvalue))
  (switch int (Utilities|Array|Length _returnvalue)
    (:1
      (Variables|Default|SetFirst "0")
      (Variables|Default|SetSecond _output))
    (:2
      (Variables|Default|SetFirst _output)
      (Variables|Default|SetSecond (Utilities|Array|Get(acopy) _returnvalue 1))))
  (return (Variables|Default|GetFirst) (Variables|Default|GetSecond)))

(fn Poweron
  (Rendering|SetVisibility (Variables|Default|GetTextRender1) true false)
  (Rendering|SetVisibility (Variables|Default|GetTextRender2) true false)
  (Variables|Default|SetEncendido true))

(fn PowerOff
  (Rendering|SetVisibility (Variables|Default|GetTextRender1) false false)
  (Rendering|SetVisibility (Variables|Default|GetTextRender2) false false)
  ;[0.04167 0.04167 0.04167] Reset the value to 0
  (Variables|Default|SetEncendido false)
  (CallFunction|SetNumbers "0" "0")
  (Variables|Default|SetValue 0)
  ;[0.04167 0.04167 0.04167] Stop the timer
  (if (Variables|Default|GetCountingDown)
    (Utilities|Time|ClearTimerbyFunctionName 0 "DecreaseValue")
    (bind _output_get (Variables|Default|SetCountingDown false))
    (Default|SetCountingDown (Variables|Default|GetNotificationManager) _output_get)))

(fn SetNumbers
  (params (First :type String) (Second :type String))
  (Rendering|Components|TextRender|SetText (Variables|Default|GetTextRender1) (Utilities|Text|ToText(String) First))
  (Rendering|Components|TextRender|SetText (Variables|Default|GetTextRender2) (Utilities|Text|ToText(String) Second)))

(fn StartTimer
  (bind _notificationmanager (Variables|Default|GetNotificationManager))
  (if (not (Variables|Default|GetCountingDown))
    (if (> (Variables|Default|GetValue) 0)
      ;[0.0625 0.0625 0.0625] Indicate that the timer has starter and notificate it
      (bind _output_get (Variables|Default|SetCountingDown true))
      (Default|SetCountingDown _notificationmanager _output_get)
      (bind _goodstart (Default|Empezar _notificationmanager))
      (if _goodstart
        (Utilities|Time|SetTimerbyFunctionName 0 "DecreaseValue" 1.0 true)
        (else
          ;[0.0625 0.0625 0.0625] Wait until the process is well done
          (bind _output_get_2 (Variables|Default|SetCountingDown false))
          (Default|SetCountingDown (Variables|Default|GetNotificationManager) _output_get_2))))))

(fn IsCountingDown
  (return (Variables|Default|GetCountingDown)))

(fn StopTimer
  (Utilities|Time|ClearTimerbyFunctionName 0 "DecreaseValue")
  (bind _output_get (Variables|Default|SetCountingDown false))
  (Default|SetCountingDown (Variables|Default|GetNotificationManager) _output_get)
  (Default|NotificateStop (Variables|Default|GetPantallaMenu)))

(fn IsMax
  (return (>= (Variables|Default|GetValue) 29)))

(fn IsMin
  (return (<= (Variables|Default|GetValue) 1)))