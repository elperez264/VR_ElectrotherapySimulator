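; Actor Blueprint that manages on-screen notifications for a procedure with an applicator and a countdown, flagging correct and incorrect step order.
; BeginPlay creates the Notifications widget and adds it to the viewport.
; Aplicar, Quitar and Empezar (apply, remove, start) check the applied and counting-down flags, triggering good or bad widget events or a debug print.
; SetCountingDown updates the countdown flag, while Apagar is an empty stub.
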(event EventBeginPlay
  (bind _returnvalue (UserInterface|CreateWidget "/Game/AppContent/UI/Notifications.Notifications_C" (Game|GetPlayerController 0)))
  (bind _output_get (Variables|Default|SetUI _returnvalue))
  (UserInterface|Viewport|AddtoViewport _output_get 0))

(event Collision|EventActorBeginOverlap
  (params (OtherActor :type Actor%20Object%20Reference)))

(event EventTick
  (params (DeltaSeconds :type Float%20%28single-precision%29)))

(fn ConstructionScript)

(fn Aplicar
  ;[0.04167 0.04167 0.04167] Si tengo una notificacion de que ha empezado sin el aplicador este mensaje sobra
  (Variables|Default|SetAplicado true)
  (if (Variables|Default|GetisCountingDown)
    (Development|PrintString "Deberias colocar el aplicador antes de empezar")))

(fn Quitar
  (if (Variables|Default|GetisCountingDown)
    (Default|MalQuitarEvent (Variables|Default|GetUI))
    (return false)
    (else
      (Variables|Default|SetAplicado false)
      (return true))))

(fn Empezar
  (bind _ui (Variables|Default|GetUI))
  (if (Variables|Default|GetisCountingDown)
    (if (Variables|Default|GetAplicado)
      (Default|BienComenzarEvent _ui)
      (return true)
      (else
        (Default|MalComenzarEvent _ui)
        (return false)))))

(fn Apagar
  (params (isCountingDown :type Boolean)))

(fn SetCountingDown
  (params (NewValue :type Boolean))
  (Variables|Default|SetisCountingDown NewValue))