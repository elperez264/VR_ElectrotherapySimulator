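; PonerAplicador is a pressable actor that toggles an applicator on and off through a Manager.
; Press calls the Manager's Aplicar or Quitar depending on the Aplicated flag, since the Manager needs that state to decide whether to start the process.
; Removal only takes effect when Quitar returns true, while applying always succeeds.
; Each successful toggle switches the text label between "Poner aplicador" and "Quitar aplicador".
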(event EventBeginPlay)

(event Collision|EventActorBeginOverlap
  (params (OtherActor :type Actor%20Object%20Reference)))

(event EventTick
  (params (DeltaSeconds :type Float%20%28single-precision%29))
  (|CallParentFunction DeltaSeconds))

(event EventPress
  (bind _manager (Variables|Default|GetManager))
  (if (Variables|Default|GetAplicated)
    ;[0.04688 0.04688 0.04688] The manager have to know if it is aplicated or not to know if have to start the process
    (bind _removewell (Default|Quitar _manager))
    (if _removewell
      (Variables|Default|SetAplicated false)
      (Rendering|Components|TextRender|SetText (Variables|Default|GetTextRender) (Utilities|Text|FormatText "Poner aplicador")))
    (else
      (Default|Aplicar _manager)
      (Variables|Default|SetAplicated true)
      (Rendering|Components|TextRender|SetText (Variables|Default|GetTextRender) (Utilities|Text|FormatText "Quitar aplicador")))))

(fn ConstructionScript)