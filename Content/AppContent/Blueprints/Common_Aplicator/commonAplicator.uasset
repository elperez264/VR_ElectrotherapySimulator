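; Common applicator Blueprint with a Cube component that tracks whether the object is applied, meaning attached.
; DesactivatePhysic turns off physics simulation on the Cube, sets the Aplicated0 flag and prints a debug message.
; Desaplicate only clears the flag and leaves physics off.
; IsAplicated and Aplicated both return that same flag, and the attachment itself happens outside these graphs.
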(event EventBeginPlay)

(event Collision|EventActorBeginOverlap
  (params (OtherActor :type Actor%20Object%20Reference)))

(event EventTick
  (params (DeltaSeconds :type Float%20%28single-precision%29)))

(event EventDesactivatePhysic
  ;[0.04688 0.04688 0.04688] Always that the phuisic are desactivated the object is attached
  (Physics|SetSimulatePhysics (Variables|Default|GetCube) false)
  (Variables|Default|Setaplicated_0 true)
  (Development|PrintString "APLICATED"))

(event EventDesaplicate
  (Variables|Default|Setaplicated_0 false))

(fn ConstructionScript)

(fn IsAplicated
  (return (Variables|Default|Getaplicated_0)))

(fn Aplicated
  (return (Variables|Default|Getaplicated_0)))