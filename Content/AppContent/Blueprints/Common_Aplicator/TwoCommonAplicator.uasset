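; Two-pole applicator actor that reports to a manager when both its Positive and Negative child applicators are applied.
; BeginPlay caches both children as commonAplicator, and Tick polls their applied state once a manager is valid.
; While both are applied it calls the manager's Aplicar every tick; losing either afterwards calls Quitar once and changes the Patient's current animation.
; SetManager stores the manager and clears its applied flag if the check does not pass.
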(event EventBeginPlay
  (bind _ascommon_aplicator (Utilities|Casting|CastTocommonAplicator (Variables|/Script/Engine.ChildActorComponent|GetChildActor (Variables|Default|GetNegative))))
  (bind _output_get (Variables|Default|SetAs%20Negative _ascommon_aplicator))
  (bind _ascommon_aplicator_2 (Utilities|Casting|CastTocommonAplicator (Variables|/Script/Engine.ChildActorComponent|GetChildActor (Variables|Default|GetPositive))))
  (bind _output_get_2 (Variables|Default|SetAs%20Positive _ascommon_aplicator_2)))

(event Collision|EventActorBeginOverlap
  (params (OtherActor :type Actor%20Object%20Reference)))

(event EventTick
  (params (DeltaSeconds :type Float%20%28single-precision%29))
  (CallFunction|CheckAplication))

(fn ConstructionScript)

(fn SetManager
  (params (NewManager :type Notification%20Manager%20Object%20Reference))
  (Variables|Default|SetManager NewManager)
  (bind _isaplicated (CallFunction|CheckAplication))
  ;[0.04688 0.04688 0.04688] confirm that the manager know that is not aplicated
  (if (not _isaplicated)
    (Variables|/Game/AppContent/Blueprints/NotificationManager.NotificationManager_C|SetAplicado (Variables|Default|GetManager) false)))

(fn CheckAplication
  ;[0.04688 0.04688 0.04688] Check that the aplicator is aplicated
  (Variables|Default|GetManager
    (:then
      (bind _isaplicated (Default|Aplicated (Variables|Default|GetAs%20Positive)))
      (bind _isaplicated_2 (Default|Aplicated (Variables|Default|GetAs%20Negative)))
      (if (and _isaplicated_2 _isaplicated)
        (Default|Aplicar (Variables|Default|GetManager))
        (bind _output_get (Variables|Default|Setaplicated true))
        (return _output_get)
        (elif (Variables|Default|Getaplicated)
          (Default|Quitar (Variables|Default|GetManager))
          (Variables|/Game/AppContent/Blueprints/NPC/NPC.NPC_C|SetactualAnimation (Variables|Default|Getpatient) "NewEnumerator2")
          (bind _output_get_2 (Variables|Default|Setaplicated false))
          (return _output_get_2))))
    (:else)))