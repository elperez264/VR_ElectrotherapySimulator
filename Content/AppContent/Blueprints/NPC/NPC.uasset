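; NPC actor that works out its current movement animation from applicators placed on its application zones.
; On BeginPlay it collects application zones from its child actor components.
; CheckAplications takes the first two colocated zones and adopts their animation if both share it and the second matches the given zone name, though every written return is false.
; Helpers gate starting on a Power limit and reset the animation on stop.
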(event EventBeginPlay
  (CallFunction|InitializeAplicationsZones))

(event Collision|EventActorBeginOverlap
  (params (OtherActor :type Actor%20Object%20Reference)))

(event EventTick
  (params (DeltaSeconds :type Float%20%28single-precision%29)))

(fn ConstructionScript)

(fn InitializeAplicationsZones
  ;[0.04688 0.04688 0.04688] Initialize the Components into aplication zones with each name. Create a new array.
  (bind _array_element (Utilities|Array|ForEachLoopwithBreak (Actor|GetComponentsByClass "/Script/Engine.ChildActorComponent"))
    (:LoopBody
      (bind _asaplication_zone (Utilities|Casting|CastToaplicationZone (Variables|/Script/Engine.ChildActorComponent|GetChildActor _array_element)))
      (Utilities|Array|Add (Variables|Default|GetaplicationZones) _asaplication_zone))))

(fn CheckAplications
  (params (zones :type aplicationZones%20Enum :default "NewEnumerator0"))
  (bind _aplicatedzones (Variables|Default|GetaplicatedZones))
  (bind _aplicationzones (Variables|Default|GetaplicationZones))
  (bind _aplicatedzones_2 (Variables|Default|GetaplicatedZones))
  (bind _output (Utilities|Array|Get(acopy) _aplicatedzones_2 1))
  (bind _output_2 (Utilities|Array|Get(acopy) _aplicationzones _output))
  (bind _movementanimation (Variables|/Game/AppContent/Blueprints/NPC/aplicationZone.aplicationZone_C|GetmovementAnimation _output_2))
  (LocalVariables|SetNewLocalVar zones)
  ;[0.04688 0.04688 0.04688] The array must be empty to do a new check
  (Utilities|Array|Clear (Variables|Default|GetaplicatedZones))
  ;[0.04688 0.04688 0.04688] Check that there are two aplicator colocated and save them
  (bind (_array_element _array_index) (Utilities|Array|ForEachLoopwithBreak (Variables|Default|GetaplicationZones) :!label _label)
    (:LoopBody
      (bind _colocated (Default|IsColocated _array_element))
      (if _colocated
        (Utilities|Array|Add _aplicatedzones _array_index)
        (if (>= (Utilities|Array|Length _aplicatedzones) 2)
          (goto _label Break))))
    (:Completed
      ;[0.04688 0.04688 0.04688] If it is the same movement in both zones, then the movement is valid
      (if (== (Utilities|Array|Length (Variables|Default|GetaplicatedZones)) 2)
        (if (Utilities|Enum|Equal(Enum) (Variables|/Game/AppContent/Blueprints/NPC/aplicationZone.aplicationZone_C|GetmovementAnimation (Utilities|Array|Get(acopy) (Variables|Default|GetaplicationZones) (Utilities|Array|Get(acopy) (Variables|Default|GetaplicatedZones)))) _movementanimation)
          (if (Utilities|Enum|Equal(Enum) (Variables|/Game/AppContent/Blueprints/NPC/aplicationZone.aplicationZone_C|GetzoneName _output_2) (LocalVariables|GetNewLocalVar))
            (Variables|Default|SetactualAnimation _movementanimation)
            (return false)
            (else
              _)))
        (return false)))))

(fn StopAplication
  (Variables|Default|SetactualAnimation "NewEnumerator2"))

(fn StartAplication
  ;[0.04688 0.04688 0.04688] Check the power to start the animation or do something before
  (if (<= (Variables|Default|GetPower) 1e+02)
    (return true)
    (else
      (return false))))