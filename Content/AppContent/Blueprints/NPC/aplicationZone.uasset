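; NPC application zone Blueprint that handles sticky applicator objects passed to it, with tick logic left to its parent class.
; CheckInterface reports whether an actor implements the StickyAplicator interface.
; PhysicsOff casts the actor to stickyAplicator, deactivates its physics and returns whether the cast succeeded.
; The Desaplicate event uses the same cast to forward removal to the applicator.
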(event EventBeginPlay)

(event Collision|EventActorBeginOverlap
  (params (OtherActor :type Actor%20Object%20Reference)))

(event EventTick
  (params (DeltaSeconds :type Float%20%28single-precision%29))
  (|CallParentFunction DeltaSeconds))

(event EventDesaplicate
  (params (NewActor :type Actor%20Object%20Reference))
  (bind _assticky_aplicator (Utilities|Casting|CastTostickyAplicator NewActor))
  (Default|Desaplicate _assticky_aplicator))

(fn ConstructionScript)

(fn PhysicsOff
  (params (NewActor :type Actor%20Object%20Reference))
  (bind _assticky_aplicator (Utilities|Casting|CastTostickyAplicator NewActor)
    (:then
      (Default|DesactivatePhysic _assticky_aplicator)
      (return true))
    (:CastFailed
      (return false))))

(fn CheckInterface
  (params (NewActor :type Actor%20Object%20Reference))
  (return (Utilities|DoesObjectImplementInterface NewActor "/Game/AppContent/Interface/stickyAplicator.stickyAplicator_C")))