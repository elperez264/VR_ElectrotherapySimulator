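; TreatmentManager is an actor Blueprint that tracks whether a treatment is currently running, allowing only one at a time.
; StartTreatment sets a CurrentlyInTreatment flag and returns true, or returns false if a treatment is already active.
; StopTreatment clears the flag and IsInTreatment exposes it, with Spanish debug strings printed on start, refusal and stop.
; The event graph and construction script contain no logic.
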(event EventBeginPlay)

(event Collision|EventActorBeginOverlap
  (params (OtherActor :type Actor%20Object%20Reference)))

(event EventTick
  (params (DeltaSeconds :type Float%20%28single-precision%29)))

(fn ConstructionScript)

(fn StartTreatment
  ;[0.04688 0.04688 0.04688] if there was a treatment running then this wont start
  (if (Variables|Default|GetcurrentlyInTreatment)
    (Development|PrintString "NO PUEDE EMPEZAR")
    (return false)
    (else
      (Variables|Default|SetcurrentlyInTreatment true)
      (Development|PrintString "EMPIEZA EL TRATAMIENTO")
      (return true))))

(fn StopTreatment
  (Variables|Default|SetcurrentlyInTreatment false)
  (Development|PrintString "ACABA EL TRATAMIENTO"))

(fn IsinTreatment
  (return (Variables|Default|GetcurrentlyInTreatment)))