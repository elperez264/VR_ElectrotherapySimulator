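; Anchor point actor that snaps an overlapping objectToAnchor actor onto itself.
; Each Tick, while it holds no valid object, it takes the first objectToAnchor in its Sphere, detaching it, or clears its state when none overlap.
; A held object gets its Cube moved to the root transform with physics off, then is attached once to the root, with debug prints throughout.
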(event EventBeginPlay)

(event Collision|EventActorBeginOverlap
  (params (OtherActor :type Actor%20Object%20Reference)))

(event EventTick
  (params (DeltaSeconds :type Float%20%28single-precision%29))
  (bind _sphere (Variables|Default|GetSphere))
  (bind _defaultsceneroot (Variables|Default|GetDefaultSceneRoot))
  (bind _overlappingactors (Collision|GetOverlappingActors _sphere "/Game/AppContent/Blueprints/Micro/Micro_Aplicator/objectToAnchor.objectToAnchor_C" :!class /Script/Engine.PrimitiveComponent))
  (bind _returnvalue (Transformation|GetWorldTransform _defaultsceneroot))
  (bind _anchorobject (Variables|Default|GetanchorObject)
    (:then
      (Development|PrintString "ES VALIDOOOOOOOOOOOOO")
      (if (not (Variables|Default|Getattached))
        (Transformation|SetWorldLocationAndRotation (Variables|/Game/AppContent/Blueprints/Micro/Micro_Aplicator/objectToAnchor.objectToAnchor_C|GetCube _anchorobject) (.location _returnvalue) (.rotation _returnvalue) false false)
        (Physics|SetSimulatePhysics (Variables|/Game/AppContent/Blueprints/Micro/Micro_Aplicator/objectToAnchor.objectToAnchor_C|GetCube (Variables|Default|GetanchorObject)) false)
        (bind _returnvalue_2 (Transformation|AttachComponentToComponent (Variables|Default|GetanchorObject) (Variables|Default|GetDefaultSceneRoot) "None" "KeepWorld" "KeepWorld" "KeepWorld" true))
        (if _returnvalue_2
          (Variables|Default|Setattached _returnvalue_2)
          (Development|PrintString "ATACHADOO"))))
    (:else
      (if (> (Utilities|Array|Length _overlappingactors) 0)
        (Utilities|IsValid (Actor|GetAttachParentActor (Variables|Default|GetanchorObject))
          (:Is%20Not%20Valid
            (Development|PrintString "ESSTAAAAAAAAA")
            (bind _asobject_to_anchor (Utilities|Casting|CastToobjectToAnchor (Utilities|Array|Get(acopy) _overlappingactors)))
            (bind _output_get (Variables|Default|SetanchorObject _asobject_to_anchor))
            (Transformation|DetachFromActor _output_get "KeepWorld" "KeepWorld" "KeepWorld")))
        (else
          (Variables|Default|SetanchorObject 0)
          (Variables|Default|Setattached false)
          (Development|PrintString "desatachado"))))))

(fn ConstructionScript)